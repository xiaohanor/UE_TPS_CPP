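; BPC_DamageSystem is a damage component that tracks health and death state for its owner.
; TakeDamage subtracts the damage info amount unless already dead, then fires OnDeath at zero or below, or OnDamage otherwise.
; Heal clamps health between zero and MaxHealth but does not check or clear the dead flag.
; Getters expose current and maximum health, and the component runs no BeginPlay or Tick logic.
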(fn `GetCurrentHealth`
  (returns (Health :type "Float (double-precision)"))
  (return (`self.Health`)))

(fn `GetMaxHealth`
  (returns (MaxHealth :type "Float (double-precision)"))
  (return (`self.MaxHealth`)))

(fn `Heal`
  (params (Amount :type "Float (double-precision)"))
  (returns (NewHealth :type "Float (double-precision)"))
  (bind _output_get (set `self.Health` (`KismetMathLibrary.FClamp` (+ Amount (`self.Health`)) 0.0 (`self.MaxHealth`))))
  (return _output_get))

(fn `TakeDamage`
  (params (DamageInfo :type "/Game/DamageSystem/S_DamageInfo Structure"))
  (returns (WasDamaged :type Boolean))
  (if (not (`self.IsDead`))
    (bind _output_get (set `self.Health` (- (`self.Health`) (`.Amount_2_D97E3D184FD0EA66BCB380AD9ACE6FBC` (break `/Game/DamageSystem/S_DamageInfo` DamageInfo)))))
    (if (<= _output_get 0.0)
      (set `self.IsDead` true)
      (`self.OnDeath`)
      (else
        (`self.OnDamage`)))
    (return true)))