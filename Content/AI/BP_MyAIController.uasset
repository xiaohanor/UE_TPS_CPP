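; AI controller that runs BT_NPC_AI and feeds player perception into its Blackboard.
; Perception updates pass through sight, prediction, hearing and touch handlers, each filtering by Player tag and sense class.
; Sight toggles 看到玩家; losing it sets NPC行为 and requests a prediction, whose stimulus supplies 玩家最后位置.
; Hearing and touch write that location directly and set the same behavior state.
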(event `self.ReceiveBeginPlay`
  (`self.RunBehaviorTree` "/Game/AI/BT_NPC_AI.BT_NPC_AI")
  (`BlackboardComponent.SetValueAsEnum` (`AIBlueprintHelperLibrary.GetBlackboard` null) "None" 0))

(event `self.AIPerception.OnTargetPerceptionUpdated`
  (params (Actor :type "Actor Object Reference") (Stimulus :type "AIStimulus Structure"))
  (`self.视力感知` Actor Stimulus)
  (`self.预感感知` Actor Stimulus)
  (`self.听力感知` Actor Stimulus)
  (`self.触摸感知` Actor Stimulus))

(fn `UserConstructionScript`)

(fn `听力感知`
  (params (Actor :type "Actor Object Reference") (AIStimulus :type "AIStimulus Structure (by ref)"))
  (bind (_age _expirationage _strength _stimuluslocation _receiverlocation _tag _bsuccessfullysensed) (break `AIStimulus` AIStimulus))
  (if (`self.ActorHasTag` Actor "Player")
    (bind _returnvalue (`AIPerceptionSystem.GetSenseClassForStimulus` AIStimulus))
    (if (== _returnvalue "/Script/AIModule.AISense_Hearing")
      (if _bsuccessfullysensed
        (`BlackboardComponent.SetValueAsVector` (`AIBlueprintHelperLibrary.GetBlackboard` null) "玩家最后位置" _stimuluslocation)
        (`BlackboardComponent.SetValueAsEnum` (`AIBlueprintHelperLibrary.GetBlackboard` null) "NPC行为" 1)
        (return)
        (else
          (return)))
      (else
        (return)))
    (else
      (return))))

(fn `视力感知`
  (params (Actor :type "Actor Object Reference") (AIStimulus :type "AIStimulus Structure (by ref)"))
  (if (`self.ActorHasTag` Actor "Player")
    (bind _returnvalue (`AIPerceptionSystem.GetSenseClassForStimulus` AIStimulus))
    (if (== _returnvalue "/Script/AIModule.AISense_Sight")
      (if (`.bSuccessfullySensed` (break `AIStimulus` AIStimulus))
        (`BlackboardComponent.SetValueAsBool` (`AIBlueprintHelperLibrary.GetBlackboard` null) "看到玩家" true)
        (else
          (`BlackboardComponent.SetValueAsBool` (`AIBlueprintHelperLibrary.GetBlackboard` null) "看到玩家" false)
          (`BlackboardComponent.SetValueAsEnum` (`AIBlueprintHelperLibrary.GetBlackboard` null) "NPC行为" 1)
          (`AISense_Prediction.RequestPawnPredictionEvent` (`self.K2_GetPawn`) (`local.Actor`) 0.5)))
      (return)
      (else
        (return)))
    (else
      (return))))

(fn `触摸感知`
  (params (Actor :type "Actor Object Reference") (AIStimulus :type "AIStimulus Structure (by ref)"))
  (bind (_age _expirationage _strength _stimuluslocation _receiverlocation _tag _bsuccessfullysensed) (break `AIStimulus` AIStimulus))
  (if (`self.ActorHasTag` Actor "Player")
    (bind _returnvalue (`AIPerceptionSystem.GetSenseClassForStimulus` AIStimulus))
    (if (== _returnvalue "/Script/AIModule.AISense_Touch")
      (if _bsuccessfullysensed
        (`BlackboardComponent.SetValueAsVector` (`AIBlueprintHelperLibrary.GetBlackboard` null) "玩家最后位置" _stimuluslocation)
        (`BlackboardComponent.SetValueAsEnum` (`AIBlueprintHelperLibrary.GetBlackboard` null) "NPC行为" 1)
        (return)
        (else
          (return)))
      (else
        (return)))
    (else
      (return))))

(fn `预感感知`
  (params (Actor :type "Actor Object Reference") (AIStimulus :type "AIStimulus Structure (by ref)"))
  (bind (_age _expirationage _strength _stimuluslocation _receiverlocation _tag _bsuccessfullysensed) (break `AIStimulus` AIStimulus))
  (if (`self.ActorHasTag` Actor "Player")
    (bind _returnvalue (`AIPerceptionSystem.GetSenseClassForStimulus` AIStimulus))
    (if (== _returnvalue "/Script/AIModule.AISense_Prediction")
      (if _bsuccessfullysensed
        (`BlackboardComponent.SetValueAsVector` (`AIBlueprintHelperLibrary.GetBlackboard` null) "玩家最后位置" _stimuluslocation)
        (return)
        (else
          (return)))
      (else
        (return)))
    (else
      (return))))